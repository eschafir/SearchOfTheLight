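; Light pickup actor that the player collects by touching it in a side-scroller.
; On sphere overlap with a Player-tagged actor, it passes its light multiplier to the SideScrollerCharacter's CollectLight, plays a pickup sound and increments the character's aura.
; It then hides itself, disables collision and waits for the sound's duration before destroying itself.
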(event OnComponentBeginOverlap(Sphere)
  (params (OverlappedComponent :type Primitive%20Component%20Object%20Reference) (OtherActor :type Actor%20Object%20Reference) (OtherComp :type Primitive%20Component%20Object%20Reference) (OtherBodyIndex :type Integer) (bFromSweep :type Boolean) (SweepResult :type Hit%20Result%20Structure%20%28by%20ref%29))
  (bind _returnvalue (Game|GetPlayerCharacter 0))
  (bind _pickupsound (Variables|Default|GetPickupSound))
  (bind _asside_scroller_character (Utilities|Casting|CastToSideScrollerCharacter _returnvalue))
  (if (Actor|ActorHasTag OtherActor "Player")
    (Default|CollectLight _asside_scroller_character (Variables|Default|GetLight%20Mutiplier))
    (Audio|Components|Audio|Play _pickupsound 0.0)
    (Default|IncrementAura _asside_scroller_character)
    (Rendering|SetActorHiddenInGame true)
    (Collision|SetActorEnableCollision false)
    (Utilities|FlowControl|Delay (Variables|/Script/Engine.SoundBase|GetDuration (Variables|/Script/Engine.AudioComponent|GetSound _pickupsound)))
    (Actor|DestroyActor)))

(fn ConstructionScript)