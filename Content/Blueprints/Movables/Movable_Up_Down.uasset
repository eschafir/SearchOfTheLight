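; Movable actor Blueprint that moves itself vertically from its starting height.
; On BeginPlay it stores the initial Z, waits a configurable InitDelay, then calls the MovementLoop event to play a timeline from the start.
; Each timeline update lerps Z between the initial height and that height plus MovementScale, keeping the current X and Y.
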(event Custom|Movement%20Loop
  (bind _returnvalue (Transformation|GetActorLocation))
  (bind _initial_z_pos (Variables|Default|GetInitial%20Z%20Pos))
  (bind _newtrack_0 (Timeline|Timeline_0 PlayFromStart)
    (:Update
      (Transformation|SetActorLocation (Math|Vector|MakeVector (.x _returnvalue) (.y _returnvalue) (Math|Float|Lerp _initial_z_pos (+ _initial_z_pos (Variables|Default|GetMovement%20Scale)) _newtrack_0)) false false))))

(event EventBeginPlay
  (Variables|Default|SetInitial%20Z%20Pos (.z (Transformation|GetActorLocation)))
  (Utilities|FlowControl|Delay (Variables|Default|GetInit%20Delay))
  (CallFunction|MovementLoop))

(fn ConstructionScript)