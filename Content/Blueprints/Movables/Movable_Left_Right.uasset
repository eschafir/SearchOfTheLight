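; Movable actor that slides along the world Y axis, offset from its starting position, as a left-right moving object.
; BeginPlay caches the starting Y and waits a configurable InitDelay before calling MovementLoop.
; MovementLoop plays a timeline from the start, whose track lerps Y between the initial position and that plus MovementScale, keeping current X and Z.
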(event Custom|Movement%20Loop
  (bind _returnvalue (Transformation|GetActorLocation))
  (bind _initial_y_pos (Variables|Default|GetInitial%20Y%20Pos))
  (bind _newtrack_0 (Timeline|Timeline_0 PlayFromStart)
    (:Update
      (Transformation|SetActorLocation (Math|Vector|MakeVector (.x _returnvalue) (Math|Float|Lerp _initial_y_pos (+ _initial_y_pos (Variables|Default|GetMovement%20Scale)) _newtrack_0) (.z _returnvalue)) false false))))

(event EventBeginPlay
  (Variables|Default|SetInitial%20Y%20Pos (.y (Transformation|GetActorLocation)))
  (Utilities|FlowControl|Delay (Variables|Default|GetInit%20Delay))
  (CallFunction|MovementLoop))

(fn ConstructionScript)